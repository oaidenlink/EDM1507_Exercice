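; MIDI manager actor that turns notes from a hardware controller into MetaSound-style synth playback.
; On BeginPlay it opens the receive-capable device whose ID matches MIDIControllerIndex, binds its MIDI event, and starts a 2D MSS_MonoSynth sound.
; Each MIDI event prints note and velocity; Note On spawns a new MSS_Synth01 2D sound with the note number as its MIDINote parameter.
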(event `self.ReceiveBeginPlay`
  (bind _outmididevices (`MIDIDeviceManager.FindMIDIDevices`))
  (for _array_element _outmididevices
    (bind (_deviceid _devicename _bcanreceivefrom) (break `FoundMIDIDevice` _array_element))
    (if _bcanreceivefrom
      (if (== (`self.MIDIControllerIndex`) _deviceid)
        (`KismetSystemLibrary.PrintString` _devicename)
        (bind _returnvalue (`MIDIDeviceManager.CreateMIDIDeviceController` _deviceid))
        (bind _output_get (set `self.MIDIControl` _returnvalue))
        (add `MIDIDeviceController.OnMIDIEvent` _output_get (`|CreateDelegate` :!event `EventOnMIDIEvent`)))))
  (`KismetSystemLibrary.PrintString` "boucle terminée")
  (bind _returnvalue_2 (`GameplayStatics.CreateSound2D` "/Game/Metasound/MSS_MonoSynth.MSS_MonoSynth" 1.0 1.0 0.0 null))
  (`AudioComponent.Play` _returnvalue_2 0.0))

(event `EventOnMIDIEvent`
  (params (MIDIDeviceController :type "MIDIDeviceController Object Reference") (Timestamp :type Integer) (EventType :type "EMIDIEventType Enum" :default "Unknown") (Channel :type Integer) (ControlID :type Integer) (Velocity :type Integer) (RawEventType :type Integer))
  (`KismetSystemLibrary.PrintString` (`KismetTextLibrary.Conv_TextToString` (`|FormatText` "MIDI Note {note} VELOCITE {velocite}" ControlID Velocity)) true true (struct :`R` 0.527637 :`G` 1.0 :`A` 1.0) 2.0 "MIDI")
  (if (`|EnumEquality` EventType "NoteOn")
    (bind _returnvalue (`GameplayStatics.CreateSound2D` "/Game/Metasound/MSS_Synth01.MSS_Synth01" 1.0 1.0 0.0 null))
    (`AudioParameterControllerInterface.SetFloatParameter` _returnvalue "MIDINote" (`KismetMathLibrary.Conv_IntToDouble` ControlID))
    (`AudioComponent.Play` _returnvalue 0.0)))

(fn `UserConstructionScript`)